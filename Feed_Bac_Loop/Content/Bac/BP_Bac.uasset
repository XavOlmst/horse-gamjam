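; BP_Bac is the visual body of the Bac character, showing one pose component at a time to match the state of a referenced BacEat actor.
; Outside Eating, Tick snaps it to BacEat's location, turns it toward the player and shows the walk, wait or scream visual.
; While Eating it stops following and switches to crumbs, setting HasEatten, only when a camera-forward dot product shows the player looking away.
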(event Custom|BacWalkEnd
  ;[0.15 0.15 0.15 0.5] Walking
  (if (not (Utilities|Enum|Equal(Enum) (Variables|/Game/Bac/BP_BacEat.BP_BacEat_C|GetBacState (Variables|Default|GetBacEat)) "NewEnumerator1"))
    (Rendering|SetVisibility (Variables|Default|GetBacStand) true false)
    (Rendering|SetVisibility (Variables|Default|GetBacCrumbs) false false)
    (Rendering|SetVisibility (Variables|Default|GetBacScream) false false)
    (Rendering|SetVisibility (Variables|Default|GetBacWait) false false)
    (Rendering|SetVisibility (Variables|Default|GetBacTalk) false false)
    (Rendering|SetVisibility (Variables|Default|GetBacWalk) false false)))

(event Custom|BacWalkStart
  ;[0.15 0.15 0.15 0.5] Walking
  (if (Utilities|Enum|Equal(Enum) (Variables|/Game/Bac/BP_BacEat.BP_BacEat_C|GetBacState (Variables|Default|GetBacEat)) "NewEnumerator1")
    (Rendering|SetVisibility (Variables|Default|GetBacStand) false false)
    (Rendering|SetVisibility (Variables|Default|GetBacCrumbs) false false)
    (Rendering|SetVisibility (Variables|Default|GetBacScream) false false)
    (Rendering|SetVisibility (Variables|Default|GetBacWait) false false)
    (Rendering|SetVisibility (Variables|Default|GetBacTalk) false false)
    (Rendering|SetVisibility (Variables|Default|GetBacWalk) true false)))

(event Custom|BacWaitStart
  ;[0.15 0.15 0.15 0.5] BacWait
  (if (Utilities|Enum|Equal(Enum) (Variables|/Game/Bac/BP_BacEat.BP_BacEat_C|GetBacState (Variables|Default|GetBacEat)) "NewEnumerator0")
    (Rendering|SetVisibility (Variables|Default|GetBacStand) false false)
    (Rendering|SetVisibility (Variables|Default|GetBacCrumbs) false false)
    (Rendering|SetVisibility (Variables|Default|GetBacScream) false false)
    (Rendering|SetVisibility (Variables|Default|GetBacWait) true false)
    (Rendering|SetVisibility (Variables|Default|GetBacTalk) false false)
    (Rendering|SetVisibility (Variables|Default|GetBacWalk) false false)))

(event Custom|BacWaitEnd
  ;[0.15 0.15 0.15 0.5] BacWait
  (if (Utilities|Enum|Equal(Enum) (Variables|/Game/Bac/BP_BacEat.BP_BacEat_C|GetBacState (Variables|Default|GetBacEat)) "NewEnumerator0")
    (Rendering|SetVisibility (Variables|Default|GetBacStand) true false)
    (Rendering|SetVisibility (Variables|Default|GetBacCrumbs) false false)
    (Rendering|SetVisibility (Variables|Default|GetBacScream) false false)
    (Rendering|SetVisibility (Variables|Default|GetBacWait) false false)
    (Rendering|SetVisibility (Variables|Default|GetBacTalk) false false)
    (Rendering|SetVisibility (Variables|Default|GetBacWalk) false false)))

(event Custom|BacScreamEnd
  ;[0.15 0.15 0.15 0.5] Screaming
  (if (Utilities|Enum|Equal(Enum) (Variables|/Game/Bac/BP_BacEat.BP_BacEat_C|GetBacState (Variables|Default|GetBacEat)) "NewEnumerator3")
    (Rendering|SetVisibility (Variables|Default|GetBacStand) true false)
    (Rendering|SetVisibility (Variables|Default|GetBacCrumbs) false false)
    (Rendering|SetVisibility (Variables|Default|GetBacScream) false false)
    (Rendering|SetVisibility (Variables|Default|GetBacWait) false false)
    (Rendering|SetVisibility (Variables|Default|GetBacTalk) false false)
    (Rendering|SetVisibility (Variables|Default|GetBacWalk) false false)))

(event Custom|BacCrumbsEnd
  ;[0.15 0.15 0.15 0.5] Crumbs
  (if (Utilities|Enum|Equal(Enum) (Variables|/Game/Bac/BP_BacEat.BP_BacEat_C|GetBacState (Variables|Default|GetBacEat)) "NewEnumerator2")
    (Rendering|SetVisibility (Variables|Default|GetBacStand) true false)
    (Rendering|SetVisibility (Variables|Default|GetBacCrumbs) false false)
    (Rendering|SetVisibility (Variables|Default|GetBacScream) false false)
    (Rendering|SetVisibility (Variables|Default|GetBacWait) false false)
    (Rendering|SetVisibility (Variables|Default|GetBacTalk) false false)
    (Rendering|SetVisibility (Variables|Default|GetBacWalk) false false)))

(event Custom|BacScreamStart
  ;[0.15 0.15 0.15 0.5] Screaming
  (if (Utilities|Enum|Equal(Enum) (Variables|/Game/Bac/BP_BacEat.BP_BacEat_C|GetBacState (Variables|Default|GetBacEat)) "NewEnumerator3")
    (Rendering|SetVisibility (Variables|Default|GetBacStand) false false)
    (Rendering|SetVisibility (Variables|Default|GetBacCrumbs) false false)
    (Rendering|SetVisibility (Variables|Default|GetBacScream) true false)
    (Rendering|SetVisibility (Variables|Default|GetBacWait) false false)
    (Rendering|SetVisibility (Variables|Default|GetBacTalk) false false)
    (Rendering|SetVisibility (Variables|Default|GetBacWalk) false false)))

(event Custom|BacCrumbsStart
  ;[0.15 0.15 0.15 0.5] Crumbs
  (if (Utilities|Enum|Equal(Enum) (Variables|/Game/Bac/BP_BacEat.BP_BacEat_C|GetBacState (Variables|Default|GetBacEat)) "NewEnumerator2")
    (Rendering|SetVisibility (Variables|Default|GetBacStand) false false)
    (Rendering|SetVisibility (Variables|Default|GetBacCrumbs) true false)
    (Rendering|SetVisibility (Variables|Default|GetBacScream) false false)
    (Rendering|SetVisibility (Variables|Default|GetBacWait) false false)
    (Rendering|SetVisibility (Variables|Default|GetBacTalk) false false)
    (Rendering|SetVisibility (Variables|Default|GetBacWalk) false false)))

(event EventBeginPlay
  ;[0.15 0.15 0.15 0.5] DefaultState
)

(event Collision|EventActorBeginOverlap
  (params (OtherActor :type Actor%20Object%20Reference)))

(event EventTick
  (params (DeltaSeconds :type Float%20%28single-precision%29))
  (if (Utilities|Enum|Equal(Enum) (Variables|/Game/Bac/BP_BacEat.BP_BacEat_C|GetBacState (Variables|Default|GetBacEat)) "NewEnumerator2")
    (if (< (Math|Vector|DotProduct (Math|Vector|GetForwardVector (Variables|/Script/Engine.PlayerCameraManager|GetTransformComponent (Game|GetPlayerCameraManager 0))) (Math|Vector|GetUnitDirection(Vector) (Transformation|GetActorLocation (Game|GetPlayerCharacter 0)) (Transformation|GetActorLocation))) 0.0)
      (Development|PrintString "Eattt")
      (switch Utilities|FlowControl|Switch|SwitchonE_BacState (Variables|/Game/Bac/BP_BacEat.BP_BacEat_C|GetBacState (Variables|Default|GetBacEat)) :!label _label
        (:NewEnumerator0
          (CallFunction|BacWaitStart))
        (:NewEnumerator1
          (CallFunction|BacWalkStart))
        (:NewEnumerator2
          (CallFunction|BacCrumbsStart)
          (Variables|Default|SethasEatten true))
        (:NewEnumerator3
          (CallFunction|BacScreamStart)))
      (else
        (Development|PrintString "LOOK AWAYYY!!!")))
    (else
      (Transformation|SetActorRotation (Math|Rotator|FindLookatRotation (Transformation|GetActorLocation) (Transformation|GetActorLocation (Game|GetPlayerCharacter 0))))
      (Transformation|SetActorLocation (Transformation|GetActorLocation (Variables|Default|GetBacEat)) false false)
      (goto _label))))

(fn ConstructionScript)