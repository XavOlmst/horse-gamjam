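; BP_BacEat is an actor that eats BP_BaseItem actors overlapping its Box, apparently wanting "loops".
; Items of the first ITEMTYPE print approval, while others print a complaint and raise BacAnger; both are destroyed.
; It then destroys itself if LoopsAte exceeds four, otherwise quits the game if BacAnger exceeds one.
; LoopsAte adds zero per accepted item, so eating never advances that counter.
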(event OnComponentBeginOverlap(Box)
  (params (OverlappedComponent :type Primitive%20Component%20Object%20Reference) (OtherActor :type Actor%20Object%20Reference) (OtherComp :type Primitive%20Component%20Object%20Reference) (OtherBodyIndex :type Integer) (bFromSweep :type Boolean) (SweepResult :type Hit%20Result%20Structure%20%28by%20ref%29))
  (bind _asbp_base_item (Utilities|Casting|CastToBP_BaseItem OtherActor))
  (Utilities|FlowControl|Sequence
    (:then_0
      (if (Utilities|Enum|Equal(Enum) (Variables|/Game/Items/BP_BaseItem.BP_BaseItem_C|GetITEM_TYPE _asbp_base_item) "NewEnumerator0")
        (Variables|Default|SetLoopsAte (+ (Variables|Default|GetLoopsAte) 0))
        (Development|PrintString "YUMMERS")
        (Actor|DestroyActor OtherActor)
        (else
          (Development|PrintString "Really dude. No loop, bro you can not be serious. You really did this to me. Man I can' believe this.")
          (Variables|Default|SetBacAnger (* (+ (Variables|Default|GetBacAnger) 1) 2))
          (Actor|DestroyActor _asbp_base_item))))
    (:then_1
      (if (> (Variables|Default|GetLoopsAte) 4)
        (Development|PrintString "Enough loop thanks bro")
        (Actor|DestroyActor)
        (elif (> (Variables|Default|GetBacAnger) 1)
          (Development|PrintString "Cringe bro get out of here. ")
          (Game|QuitGame 0 "Quit" false))))))

(fn ConstructionScript)