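; Base interactable Blueprint that shows a widget while looked at and responds to the E key.
; LookAt reveals the widget and sets a flag that Tick clears each frame, so the widget hides via LookAway unless LookAt keeps being called.
; While flagged, Tick yaws the widget toward the player character.
; E calls Interact when the flag is set, which only prints a debug string here.
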(event Custom|Interact
  (Development|PrintString "Interacted with Object"))

(event EventTick
  (params (DeltaSeconds :type Float%20%28single-precision%29))
  (if (Variables|Default|GethasBeenLookedAt)
    (Variables|Default|SethasBeenLookedAt false)
    (Transformation|SetWorldRotation (Variables|Default|GetWidget1) (Math|Rotator|MakeRotator 0.0 0.0 (.yaw (Math|Rotator|FindLookatRotation (Transformation|GetWorldLocation (Variables|Default|GetWidget1)) (Transformation|GetActorLocation (Game|GetPlayerCharacter 0))))) false false)
    (else
      (CallFunction|LookAway))))

(event Input|KeyboardEvents|E
  (params (Key :type Key%20Structure :default "None"))
  (:Pressed
    (if (Variables|Default|GethasBeenLookedAt)
      (CallFunction|Interact))))

(fn ConstructionScript)

(fn Lookat
  (Rendering|SetVisibility (Variables|Default|GetWidget1) true true)
  (Variables|Default|SethasBeenLookedAt true))

(fn LookAway
  (Rendering|SetVisibility (Variables|Default|GetWidget1) false true))