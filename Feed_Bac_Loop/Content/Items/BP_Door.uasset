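; BP_Door is a swinging door that can be toggled by interaction or opened automatically for BP_Bac actors.
; The DoorMovement timeline drives the Cube's relative yaw, playing to open and reversing to close.
; Interact flips IsOpen to choose the direction.
; BacDoor overlap begin and end open and close the door for BP_Bac without updating IsOpen.
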(event OnComponentBeginOverlap(BacDoor)
  (params (OverlappedComponent :type Primitive%20Component%20Object%20Reference) (OtherActor :type Actor%20Object%20Reference) (OtherComp :type Primitive%20Component%20Object%20Reference) (OtherBodyIndex :type Integer) (bFromSweep :type Boolean) (SweepResult :type Hit%20Result%20Structure%20%28by%20ref%29))
  (Utilities|Casting|CastToBP_Bac OtherActor)
  (CallFunction|OpenDoor))

(event OnComponentEndOverlap(BacDoor)
  (params (OverlappedComponent :type Primitive%20Component%20Object%20Reference) (OtherActor :type Actor%20Object%20Reference) (OtherComp :type Primitive%20Component%20Object%20Reference) (OtherBodyIndex :type Integer))
  (Utilities|Casting|CastToBP_Bac OtherActor)
  (CallFunction|CloseDoor))

(event Custom|CloseDoor
  (bind _rotation (Timeline|DoorMovement Reverse)
    (:Update
      (Transformation|SetRelativeRotation (Variables|Default|GetCube) (Math|Rotator|MakeRotator 0.0 0.0 (.z _rotation)) false false))))

(event Custom|OpenDoor
  (bind _rotation (Timeline|DoorMovement Play)
    (:Update
      (Transformation|SetRelativeRotation (Variables|Default|GetCube) (Math|Rotator|MakeRotator 0.0 0.0 (.z _rotation)) false false))))

(event EventBeginPlay)

(event Collision|EventActorBeginOverlap
  (params (OtherActor :type Actor%20Object%20Reference)))

(event EventTick
  (params (DeltaSeconds :type Float%20%28single-precision%29))
  (|CallParentFunction DeltaSeconds) ; This node is disabled and will not be called.\nDrag off pins to build functionality.
)

(event EventInteract
  (bind _output_get (Variables|Default|SetisOpen (not (Variables|Default|GetisOpen))))
  (if _output_get
    (CallFunction|OpenDoor)
    (else
      (CallFunction|CloseDoor))))

(fn ConstructionScript
  (|CallParentFunction))