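; BP_CabinetDoors is an interactable cabinet whose two doors swing open and closed.
; Each Interact event toggles IsOpen, then plays or reverses the Movement timeline.
; The timeline's ZRot track sets the relative yaw of Cube and Cube1 in opposite directions, so the doors mirror each other.
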(event EventBeginPlay)

(event Collision|EventActorBeginOverlap
  (params (OtherActor :type Actor%20Object%20Reference)))

(event EventTick
  (params (DeltaSeconds :type Float%20%28single-precision%29))
  (|CallParentFunction DeltaSeconds) ; This node is disabled and will not be called.\nDrag off pins to build functionality.
)

(event EventInteract
  (bind _output_get (Variables|Default|SetisOpen (not (Variables|Default|GetisOpen))))
  (if _output_get
    (bind _z_rot (Timeline|Movement Play)
      (:Update
        (Utilities|FlowControl|Sequence
          (:then_0
            (Transformation|SetRelativeRotation (Variables|Default|GetCube) (Math|Rotator|MakeRotator 0.0 0.0 (* _z_rot -1.0)) false false))
          (:then_1
            (Transformation|SetRelativeRotation (Variables|Default|GetCube1) (Math|Rotator|MakeRotator 0.0 0.0 _z_rot) false false)))))
    (else
      (Timeline|Movement Reverse))))

(fn ConstructionScript
  (|CallParentFunction))