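; BP_BaseItem is a base item Blueprint that flags its Cube component for highlighting while it is looked at.
; Lookat and LookAway call their parent versions, then switch the Cube's Render Custom Depth on and off, which a custom-depth post-process effect can use.
; The construction script only calls the parent, and BeginPlay, overlap and Tick are unused.
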(event EventBeginPlay)

(event Collision|EventActorBeginOverlap
  (params (OtherActor :type Actor%20Object%20Reference)))

(event EventTick
  (params (DeltaSeconds :type Float%20%28single-precision%29))
  (|CallParentFunction DeltaSeconds) ; This node is disabled and will not be called.\nDrag off pins to build functionality.
)

(event EventLookat
  (|CallParentFunction)
  (Rendering|SetRenderCustomDepth (Variables|Default|GetCube) true))

(event EventLookAway
  (|CallParentFunction)
  (Rendering|SetRenderCustomDepth (Variables|Default|GetCube) false))

(fn ConstructionScript
  (|CallParentFunction))